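; 2D Paper sprite player that takes its control values from an Arduino over a serial COM port.
; BeginPlay pauses the game with the cursor shown, switches to unlit view and opens the port, which EndPlay closes.
; Tick writes to the board, then after a short delay parses letter-tagged readings into left/right speed and jump height variables, and turns the sprite toward the greater speed.
; P opens the pause menu.
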(event `self.ReceiveBeginPlay`
  (`|ExecutionSequence`
    (:`then_0`
      ;[1 1 1] Show cursor + pause game + unlit
      (set `PlayerController.bShowMouseCursor` true (`GameplayStatics.GetPlayerController` 0))
      (`GameplayStatics.SetGamePaused` true)
      (`KismetSystemLibrary.ExecuteConsoleCommand` "viewmode unlit"))
    (:`then_2`
      ;[1 1 1] Connect Arduino
      (bind (_bopened _returnvalue) (`Serial.OpenComPort` 5 19200))
      (if _bopened
        (bind _output_get (set `self.Arduino` _returnvalue))
        (`Serial.Flush` _output_get)
        (else
          (`KismetSystemLibrary.PrintString` "Port not opened"))))))

(event `self.ReceiveEndPlay`
  (params (EndPlayReason :type "EEndPlayReason Enum" :default "Destroyed"))
  (bind _arduino (`self.Arduino`))
  ;[1 1 1] Connect Arduino
  (`/Engine/EditorBlueprintResources/StandardMacros.IsValid` _arduino
    (:`Is Valid`
      (`Serial.Close` _arduino))))

(event `self.ReceiveTick`
  (params (DeltaSeconds :type "Float (single-precision)"))
  (bind _papersprite (`self.PaperSprite`))
  (bind _arduino (`self.Arduino`))
  (`|ExecutionSequence`
    (:`then_0`
      ;[1 1 1] Applying speed
      (`/Engine/EditorBlueprintResources/StandardMacros.IsValid` _arduino
        (:`Is Valid`
          (`Serial.Print` _arduino "string")
          (`KismetSystemLibrary.Delay` 0.1)
          (bind (_bsuccess _returnvalue) (`Serial.ReadString` _arduino))
          (`|ExecutionSequence`
            (:`then_0`
              (set `self.RightSpeed` (`KismetStringLibrary.Conv_StringToDouble` (`.RightS` (`KismetStringLibrary.Split` _returnvalue "r" "CaseSensitive")))))
            (:`then_1`
              (set `self.LeftSpeed` (`KismetStringLibrary.Conv_StringToDouble` (`.RightS` (`KismetStringLibrary.Split` _returnvalue "l" "CaseSensitive")))))
            (:`then_2`
              (set `self.JumpHeight` (`KismetStringLibrary.Conv_StringToDouble` (`.RightS` (`KismetStringLibrary.Split` _returnvalue "j" "CaseSensitive"))))))
          (`Serial.Flush` _arduino))))
    (:`then_1`
      ;[1 1 1] Change sprite direction
      (if (> (`self.LeftSpeed`) (`self.RightSpeed`))
        (`SceneComponent.K2_SetRelativeRotation` _papersprite (struct :`Yaw` 180.0) false false)
        (else
          (`SceneComponent.K2_SetRelativeRotation` :`self` _papersprite))))))

(event `Key|P`
  (params (Key :type "Key Structure"))
  ;[1 1 1] Pause game
  (:`Pressed`
    (bind _returnvalue (`|CreateWidget` "/Game/Blueprints/PauseMenuWidget.PauseMenuWidget_C"))
    (`UserWidget.AddToViewport` _returnvalue 0)
    (`GameplayStatics.SetGamePaused` true)
    (set `PlayerController.bShowMouseCursor` true (`GameplayStatics.GetPlayerController` 0))))

(fn `UserConstructionScript`)