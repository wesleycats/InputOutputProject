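; GameControllerBP1 is a game controller that runs a minutes-and-seconds countdown and opens the "Main" level when time runs out.
; Tick feeds a one-second Delay, which throttles the decrement to roughly once per second.
; When Seconds reaches zero it resets to 59 and Minutes drops by one, and a negative Minutes value triggers the level load.
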(event `self.ReceiveTick`
  (params (DeltaSeconds :type "Float (single-precision)"))
  ;[1 1 1] timer
  (`KismetSystemLibrary.Delay` 1.0)
  (set `self.Seconds` (- (`self.Seconds`) 1))
  (if (== (`self.Seconds`) 0)
    (set `self.minutes` (- (`self.minutes`) 1))
    (set `self.Seconds` 59))
  (if (< (`self.minutes`) 0)
    (if (< (`self.minutes`) 0)
      (`GameplayStatics.OpenLevel` "Main"))))

(fn `UserConstructionScript`)