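; Player Blueprint for a Paper2D game controlled by an Arduino over a serial port.
; Tick parses serial strings into left/right speed, jump height and pause values, flips the sprite, and creates a new hidden pause widget every frame.
; Space or the Arduino pauses; falling too low or pressing T returns to the last checkpoint.
; Overlaps save name-matched checkpoints, and hitting a named Joey sprite shows the win widget.
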(event `self.ReceiveBeginPlay`
  (`|ExecutionSequence`
    (:`then_0`
      ;[1 1 1] Set respawn position
      (set `self.RespawnPosition` (`self.K2_GetActorLocation`)))
    (:`then_1`
      ;[1 1 1] Setup
      (set `PlayerController.bShowMouseCursor` true (`GameplayStatics.GetPlayerController` 0))
      (`GameplayStatics.SetGamePaused` true)
      (`KismetSystemLibrary.ExecuteConsoleCommand` "viewmode unlit"))
    (:`then_2`
      ;[1 1 1] Connect Arduino
      (bind (_bopened _returnvalue) (`Serial.OpenComPort` 5 19200))
      (if _bopened
        (bind _output_get (set `self.Arduino` _returnvalue))
        (`Serial.Flush` _output_get)
        (else
          (`KismetSystemLibrary.PrintString` "Port not opened"))))))

(event `self.ReceiveEndPlay`
  (params (EndPlayReason :type "EEndPlayReason Enum" :default "Destroyed"))
  (bind _arduino (`self.Arduino`))
  ;[1 1 1] Connect Arduino
  (`/Engine/EditorBlueprintResources/StandardMacros.IsValid` _arduino
    (:`Is Valid`
      (`Serial.Close` _arduino))))

(event `Key|SpaceBar`
  (params (Key :type "Key Structure"))
  ;[1 1 1] Pause Game
  (:`Pressed`
    (`/Engine/EditorBlueprintResources/StandardMacros.FlipFlop`
      (:`A`
        (set `self.Paused` true)
        (`Widget.SetVisibility` (`self.PauseMenu`) "Visible" :!label _label)
        (`GameplayStatics.SetGamePaused` true)
        (set `PlayerController.bShowMouseCursor` true (`GameplayStatics.GetPlayerController` 0))
        (`/Engine/EditorBlueprintResources/StandardMacros.IsValid` (`self.Arduino`)
          (:`Is Valid`
            (`Serial.Flush` (`self.Arduino`))))))))

(event `self.ReceiveTick`
  (params (DeltaSeconds :type "Float (single-precision)"))
  (bind _papersprite (`self.PaperSprite`))
  (bind _arduino (`self.Arduino`))
  (`|ExecutionSequence`
    (:`then_0`
      ;[1 1 1] Reading data from arduino
      (`/Engine/EditorBlueprintResources/StandardMacros.IsValid` _arduino
        (:`Is Valid`
          (`Serial.Print` _arduino "string")
          (`KismetSystemLibrary.Delay` 0.1)
          (bind (_bsuccess _returnvalue) (`Serial.ReadString` _arduino))
          (`|ExecutionSequence`
            (:`then_0`
              ;[1 1 1] Applying speed to player
              (`|ExecutionSequence`
                (:`then_0`
                  (set `self.RightSpeed` (`KismetStringLibrary.Conv_StringToDouble` (`.RightS` (`KismetStringLibrary.Split` _returnvalue "r" "CaseSensitive")))))
                (:`then_1`
                  (set `self.LeftSpeed` (`KismetStringLibrary.Conv_StringToDouble` (`.RightS` (`KismetStringLibrary.Split` _returnvalue "l" "CaseSensitive")))))
                (:`then_2`
                  (set `self.JumpHeight` (`KismetStringLibrary.Conv_StringToDouble` (`.RightS` (`KismetStringLibrary.Split` _returnvalue "j" "CaseSensitive"))))))
              (`Serial.Flush` _arduino))
            (:`then_1`
              ;[1 1 1] Pause Game
              (if (== (`KismetStringLibrary.Conv_StringToInt` (`.RightS` (`KismetStringLibrary.Split` _returnvalue "p" "CaseSensitive"))) 1)
                (`/Engine/EditorBlueprintResources/StandardMacros.DoOnce` false
                  (:`Completed`
                    (goto _label)))))))))
    (:`then_1`
      ;[1 1 1] Create pause menu
      (bind _returnvalue_2 (`|CreateWidget` "/Game/Blueprints/PauseMenuWidget.PauseMenuWidget_C"))
      (bind _output_get (set `self.PauseMenu` _returnvalue_2))
      (`UserWidget.AddToViewport` _output_get 0)
      (`Widget.SetVisibility` _output_get "Hidden"))
    (:`then_2`
      ;[1 1 1] Change sprite direction
      (if (> (`self.LeftSpeed`) (`self.RightSpeed`))
        (`SceneComponent.K2_SetRelativeRotation` _papersprite (struct :`Yaw` 180.0) false false)
        (else
          (`SceneComponent.K2_SetRelativeRotation` :`self` _papersprite))))
    (:`then_3`
      ;[1 1 1] Respawn
      (`/Engine/EditorBlueprintResources/StandardMacros.CompareFloat` -1500.0 (.z (`self.K2_GetActorLocation`))
        (:`>`
          (`self.K2_SetActorLocation` (`self.RespawnPosition`) false true :!label _label_2))))))

(event `Key|T`
  (params (Key :type "Key Structure"))
  ;[1 1 1] Respawn
  (:`Pressed`
    (goto _label_2)))

(event `self.ReceiveActorBeginOverlap`
  (params (OtherActor :type "Actor Object Reference"))
  (bind _returnvalue (`self.K2_GetActorLocation` OtherActor))
  (bind _returnvalue_2 (`KismetSystemLibrary.GetObjectName` OtherActor))
  ;[1 1 1] Checkpoint collision check
  (bind _returnvalue_3 (`AddComponent|NODE_AddPaperSpriteComponent-1` :`self` OtherActor))
  (bind _returnvalue_4 (`PaperSpriteComponent.SetSprite` _returnvalue_3 "/Game/Art/Sprites/checkpoint-reached_Sprite.checkpoint-reached_Sprite"))
  (`PrimitiveComponent.SetCollisionEnabled` _returnvalue_3 "NoCollision")
  (if _returnvalue_4
    (`|ExecutionSequence`
      (:`then_0`
        (if (`KismetStringLibrary.EqualEqual_StrStr` _returnvalue_2 "checkpoint_1")
          (set `self.RespawnPosition` _returnvalue)))
      (:`then_1`
        (if (`KismetStringLibrary.EqualEqual_StrStr` _returnvalue_2 "checkpoint2_3")
          (set `self.RespawnPosition` _returnvalue)))
      (:`then_2`
        (if (`KismetStringLibrary.EqualEqual_StrStr` _returnvalue_2 "checkpoint3")
          (set `self.RespawnPosition` _returnvalue)))
      (:`then_3`
        (if (`KismetStringLibrary.EqualEqual_StrStr` _returnvalue_2 "checkpoint4")
          (set `self.RespawnPosition` _returnvalue))))))

(event `self.ReceiveHit`
  (params (MyComp :type "PrimitiveComponent Object Reference") (Other :type "Actor Object Reference") (OtherComp :type "PrimitiveComponent Object Reference") (bSelfMoved :type Boolean) (HitLocation :type "Vector Structure") (HitNormal :type "Vector Structure") (NormalImpulse :type "Vector Structure") (Hit :type "HitResult Structure (by ref)"))
  (bind _returnvalue (`KismetSystemLibrary.GetObjectName` Other))
  ;[1 1 1] Joey collision check
  (`|ExecutionSequence`
    (:`then_0`
      (if (`KismetStringLibrary.EqualEqual_StrStr` _returnvalue "Joey-Sprite2")
        (bind _returnvalue_2 (`|CreateWidget` "/Game/Blueprints/WinWidget.WinWidget_C" :!label _label_3))
        (`UserWidget.AddToViewport` _returnvalue_2 0)
        (`Widget.SetVisibility` _returnvalue_2 "Visible")))
    (:`then_1`
      (if (`KismetStringLibrary.EqualEqual_StrStr` _returnvalue "Joey-Sprite_5")
        (goto _label_3)))))

(fn `UserConstructionScript`)